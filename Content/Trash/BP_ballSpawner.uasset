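; BP_ballSpawner is an actor that repeatedly spawns BP_ball physics balls at its own location.
; BeginPlay starts the custom spawn event, which creates a ball and launches its Sphere with a random impulse along the positive X, Y and Z axes.
; After a fixed Delay the event calls itself again, forming an endless timed loop with no spawn limit or cleanup in this Blueprint.
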(event `self.ReceiveBeginPlay`
  (`self.spawn`))

(event `spawn`
  (bind _returnvalue (`|SpawnActorFromClass` "/Game/Blueprints/BP_ball.BP_ball_C" (`KismetMathLibrary.MakeTransform` (`self.K2_GetActorLocation`)) "Undefined" "MultiplyWithRoot" null null))
  (`PrimitiveComponent.AddImpulse` (`/Game/Blueprints/BP_ball.Sphere` _returnvalue) (`KismetMathLibrary.MakeVector` (`KismetMathLibrary.RandomFloatInRange` 0.0 10000.0) (`KismetMathLibrary.RandomFloatInRange` 0.0 10000.0) (`KismetMathLibrary.RandomFloatInRange` 0.0 10000.0)) "None" false)
  (`KismetSystemLibrary.Delay` 15.0)
  (`self.spawn`))

(fn `UserConstructionScript`)