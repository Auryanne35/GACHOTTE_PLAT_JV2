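; BP_masterCube is a cube actor that is either safe or deadly, set by its Good flag.
; Any overlap with its Box on a non-Good cube calls Death on player 0's character, without checking which actor overlapped.
; The changeColor event reads the character's ChangeCube flag to reveal the path, tinting Good cubes green and others red, or all white when off.
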(event `self.ReceiveBeginPlay`)

(event `self.ReceiveTick`
  (params (DeltaSeconds :type "Float (single-precision)")))

(event `self.Box.OnComponentBeginOverlap`
  (params (OverlappedComponent :type "PrimitiveComponent Object Reference") (OtherActor :type "Actor Object Reference") (OtherComp :type "PrimitiveComponent Object Reference") (OtherBodyIndex :type Integer) (bFromSweep :type Boolean) (SweepResult :type "HitResult Structure (by ref)"))
  (if (not (`self.good`))
    (bind _asbp_third_person_character (cast `/Game/Base_unreal/ThirdPerson/Blueprints/BP_ThirdPersonCharacter` (`GameplayStatics.GetPlayerCharacter` 0)))
    (`/Game/Base_unreal/ThirdPerson/Blueprints/BP_ThirdPersonCharacter.death` _asbp_third_person_character)))

(event `changeColor`
  ; Change color when player see the way
  (bind _asbp_third_person_character (cast `/Game/Base_unreal/ThirdPerson/Blueprints/BP_ThirdPersonCharacter` (`GameplayStatics.GetPlayerCharacter` 0)))
  (if (`/Game/Base_unreal/ThirdPerson/Blueprints/BP_ThirdPersonCharacter.changeCube` _asbp_third_person_character)
    (if (`self.good`)
      (`MeshComponent.SetColorParameterValueOnMaterials` (`self.Cube`) "color" (struct :`R` 0.023293 :`G` 1.0 :`A` 1.0))
      (else
        (`MeshComponent.SetColorParameterValueOnMaterials` (`self.Cube`) "color" (struct :`R` 1.0 :`G` 0.005397 :`A` 1.0))))
    (else
      (`MeshComponent.SetColorParameterValueOnMaterials` (`self.Cube`) "color" (struct :`R` 1.0 :`G` 1.0 :`B` 1.0 :`A` 1.0)))))

(fn `UserConstructionScript`)