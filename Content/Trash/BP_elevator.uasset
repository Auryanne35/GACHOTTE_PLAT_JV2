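; BP_elevator is an elevator that moves its Cube between its relative origin and a Deplacement offset.
; Overlapping the Box toggles the Place flag and either plays the Elevation timeline from start or reverses it, with the timeline's track driving a lerp of the Cube's relative location.
; Leaving the Box clears CanMove for TimeWait seconds, blocking retriggering during that delay.
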(event `self.Box.OnComponentBeginOverlap`
  (params (OverlappedComponent :type "PrimitiveComponent Object Reference") (OtherActor :type "Actor Object Reference") (OtherComp :type "PrimitiveComponent Object Reference") (OtherBodyIndex :type Integer) (bFromSweep :type Boolean) (SweepResult :type "HitResult Structure (by ref)"))
  (if (`self.canMove`)
    (if (`self.place`)
      (set `self.place` false)
      (bind (_direction _newtrack_0) (`Timeline|elevation` :!via `PlayFromStart` :!label _label)
        (:`Update`
          (`SceneComponent.K2_SetRelativeLocation` (`self.Cube`) (`KismetMathLibrary.VLerp` (0.0 0.0 0.0) (`self.deplacement`) _newtrack_0) false false)))
      (else
        (set `self.place` true)
        (goto _label :!via `Reverse`)))))

(event `self.Box.OnComponentEndOverlap`
  (params (OverlappedComponent :type "PrimitiveComponent Object Reference") (OtherActor :type "Actor Object Reference") (OtherComp :type "PrimitiveComponent Object Reference") (OtherBodyIndex :type Integer))
  (set `self.canMove` false)
  (`KismetSystemLibrary.Delay` (`self.TimeWait`))
  (set `self.canMove` true))

(fn `UserConstructionScript`)