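; A bumper obstacle that swings back and forth and knocks the third-person player character on contact.
; From BeginPlay, Turn alternates playing and reversing a timeline that lerps the SMBump mesh's relative rotation, calling itself on finish to loop.
; The Run flag tracks swing direction, so a character overlapping the Box gets a large movement impulse forward or backward along the Arrow accordingly.
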(event `self.ReceiveTick`
  (params (DeltaSeconds :type "Float (single-precision)")))

(event `self.ReceiveBeginPlay`
  (`self.turn`))

(event `turn`
  ; Function to move the asset
  (if (`self.run`)
    (set `self.run` false)
    (bind (_direction _newtrack_0) (`Timeline|Timeline` :!via `PlayFromStart` :!label _label)
      (:`Update`
        (`SceneComponent.K2_SetRelativeRotation` (`self.SM_bump`) (`KismetMathLibrary.RLerp` (struct) (`self.rotate`) _newtrack_0) false false))
      (:`Finished`
        (`self.turn`)))
    (else
      (set `self.run` true)
      (goto _label :!via `Reverse`))))

(event `self.Box.OnComponentBeginOverlap`
  (params (OverlappedComponent :type "PrimitiveComponent Object Reference") (OtherActor :type "Actor Object Reference") (OtherComp :type "PrimitiveComponent Object Reference") (OtherBodyIndex :type Integer) (bFromSweep :type Boolean) (SweepResult :type "HitResult Structure (by ref)"))
  ; Bump player
  (if (`self.run`)
    (bind _asbp_third_person_character (cast `/Game/Base_unreal/ThirdPerson/Blueprints/BP_ThirdPersonCharacter` OtherActor))
    (`CharacterMovementComponent.AddImpulse` (`Character.CharacterMovement` _asbp_third_person_character) (* (`SceneComponent.GetForwardVector` (`self.Arrow`)) -100000.0) false)
    (else
      (bind _asbp_third_person_character_2 (cast `/Game/Base_unreal/ThirdPerson/Blueprints/BP_ThirdPersonCharacter` OtherActor))
      (`CharacterMovementComponent.AddImpulse` (`Character.CharacterMovement` _asbp_third_person_character_2) (* (`SceneComponent.GetForwardVector` (`self.Arrow`)) 100000.0) false))))

(fn `UserConstructionScript`)