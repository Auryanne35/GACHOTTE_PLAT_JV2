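; BP_ball is a ball actor that randomizes its size and color when play begins.
; On BeginPlay it multiplies the actor scale by a random factor and applies it as the Sphere component's world scale.
; It then sets the "color" material parameter on the Sphere to a fully random RGBA value.
; The overlap, tick and construction script graphs are empty.
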(event `self.ReceiveBeginPlay`
  (`SceneComponent.SetWorldScale3D` (`self.Sphere`) (* (`self.GetActorScale3D`) (`KismetMathLibrary.RandomFloatInRange` 0.5 3.0)))
  (`MeshComponent.SetColorParameterValueOnMaterials` (`self.Sphere`) "color" (`KismetMathLibrary.MakeColor` (`KismetMathLibrary.RandomFloatInRange` 0.0 1.0) (`KismetMathLibrary.RandomFloatInRange` 0.0 1.0) (`KismetMathLibrary.RandomFloatInRange` 0.0 1.0) (`KismetMathLibrary.RandomFloatInRange` 0.0 1.0))))

(fn `UserConstructionScript`)