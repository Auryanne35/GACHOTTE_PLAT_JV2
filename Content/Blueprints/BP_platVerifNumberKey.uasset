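; A key-check plate that opens a linked Door when the third-person character has enough keys.
; At start its text is prefixed with the required count, and each tick it rotates toward the player's follow camera.
; Overlapping the box deducts the keys, raises the door's cube via a timeline and shows "Is Good".
; With too few keys the text turns red until overlap ends.
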(event `self.ReceiveBeginPlay`
  (bind _textrender (`self.TextRender`))
  ; Set text at the begin
  (`TextRenderComponent.K2_SetText` _textrender (`KismetTextLibrary.Conv_StringToText` (`KismetStringLibrary.Concat_StrStr` (`KismetTextLibrary.Conv_TextToString` (`KismetTextLibrary.Conv_IntToText` (`self.NecessaryKeys`))) (`KismetTextLibrary.Conv_TextToString` (`TextRenderComponent.Text` _textrender))))))

(event `self.ReceiveTick`
  (params (DeltaSeconds :type "Float (single-precision)"))
  (bind _textrender (`self.TextRender`))
  ; Set the text in front of camera
  (bind _asbp_third_person_character (cast `/Game/Base_unreal/ThirdPerson/Blueprints/BP_ThirdPersonCharacter` (`GameplayStatics.GetPlayerCharacter` 0)))
  (`SceneComponent.K2_SetRelativeRotation` _textrender (`KismetMathLibrary.FindRelativeLookAtRotation` (`KismetMathLibrary.Conv_VectorToTransform` (`SceneComponent.K2_GetComponentLocation` _textrender)) (`SceneComponent.K2_GetComponentLocation` (`/Game/Base_unreal/ThirdPerson/Blueprints/BP_ThirdPersonCharacter.FollowCamera` _asbp_third_person_character))) false false))

(event `self.Box.OnComponentBeginOverlap`
  (params (OverlappedComponent :type "PrimitiveComponent Object Reference") (OtherActor :type "Actor Object Reference") (OtherComp :type "PrimitiveComponent Object Reference") (OtherBodyIndex :type Integer) (bFromSweep :type Boolean) (SweepResult :type "HitResult Structure (by ref)"))
  (bind _necessarykeys (`self.NecessaryKeys`))
  ; Verif number of key and set color of text
  (bind _asbp_third_person_character (cast `/Game/Base_unreal/ThirdPerson/Blueprints/BP_ThirdPersonCharacter` OtherActor))
  (bind _keys (`/Game/Base_unreal/ThirdPerson/Blueprints/BP_ThirdPersonCharacter.keys` _asbp_third_person_character))
  (if (>= _keys _necessarykeys)
    (set `/Game/Base_unreal/ThirdPerson/Blueprints/BP_ThirdPersonCharacter.keys` (- _keys _necessarykeys) _asbp_third_person_character)
    (bind (_direction _newtrack_0) (`Timeline|Open`)
      (:`Update`
        (`SceneComponent.K2_SetRelativeLocation` (`/Game/Blueprints/BP_door.Cube` (`self.door`)) (`KismetMathLibrary.VLerp` (0.0 0.0 0.0) (0.0 0.0 70.0) _newtrack_0) false false)
        (`TextRenderComponent.K2_SetText` (`self.TextRender`) (`KismetTextLibrary.Conv_StringToText` "Is Good"))))
    (else
      (`TextRenderComponent.SetTextRenderColor` (`self.TextRender`) (make `Color` 0 0 255)))))

(event `self.Box.OnComponentEndOverlap`
  (params (OverlappedComponent :type "PrimitiveComponent Object Reference") (OtherActor :type "Actor Object Reference") (OtherComp :type "PrimitiveComponent Object Reference") (OtherBodyIndex :type Integer))
  ; Reset color
  (`TextRenderComponent.SetTextRenderColor` (`self.TextRender`) (make `Color` 197 255 144)))

(fn `UserConstructionScript`)