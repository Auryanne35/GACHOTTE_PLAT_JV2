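; BP_arrowsPlatform is a platform that moves along X or Y in response to overlaps with its directional boxes.
; Four direction boxes set a fixed step vector, which Tick adds to the location each frame without delta-time scaling or sweep.
; Four matching stop boxes zero that vector and nudge the platform slightly along their axis, with the same sign as their direction box.
; Overlaps are not filtered by actor.
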(event `StopMove`
  (params (Teleport :type "Vector Structure"))
  (set `self.SetMove` (0.0 0.0 0.0))
  (`self.K2_SetActorLocation` (+ (`self.K2_GetActorLocation`) Teleport)))

(event `Move`
  (params (NewLocation :type "Vector Structure"))
  (`self.K2_SetActorLocation` (+ (`self.K2_GetActorLocation`) NewLocation)))

(event `self.ReceiveTick`
  (params (DeltaSeconds :type "Float (single-precision)"))
  (`self.Move` (`self.SetMove`)))

(event `self.Box_back.OnComponentBeginOverlap`
  (params (OverlappedComponent :type "PrimitiveComponent Object Reference") (OtherActor :type "Actor Object Reference") (OtherComp :type "PrimitiveComponent Object Reference") (OtherBodyIndex :type Integer) (bFromSweep :type Boolean) (SweepResult :type "HitResult Structure (by ref)"))
  ; Choix direction
  (set `self.SetMove` (2.0 0.0 0.0)))

(event `self.Box_left.OnComponentBeginOverlap`
  (params (OverlappedComponent :type "PrimitiveComponent Object Reference") (OtherActor :type "Actor Object Reference") (OtherComp :type "PrimitiveComponent Object Reference") (OtherBodyIndex :type Integer) (bFromSweep :type Boolean) (SweepResult :type "HitResult Structure (by ref)"))
  ; Choix direction
  (set `self.SetMove` (0.0 2.0 0.0)))

(event `self.Box_front.OnComponentBeginOverlap`
  (params (OverlappedComponent :type "PrimitiveComponent Object Reference") (OtherActor :type "Actor Object Reference") (OtherComp :type "PrimitiveComponent Object Reference") (OtherBodyIndex :type Integer) (bFromSweep :type Boolean) (SweepResult :type "HitResult Structure (by ref)"))
  ; Choix direction
  (set `self.SetMove` (-2.0 0.0 0.0)))

(event `self.Box_right.OnComponentBeginOverlap`
  (params (OverlappedComponent :type "PrimitiveComponent Object Reference") (OtherActor :type "Actor Object Reference") (OtherComp :type "PrimitiveComponent Object Reference") (OtherBodyIndex :type Integer) (bFromSweep :type Boolean) (SweepResult :type "HitResult Structure (by ref)"))
  ; Choix direction
  (set `self.SetMove` (0.0 -2.0 0.0)))

(event `self.box_stop_back.OnComponentBeginOverlap`
  (params (OverlappedComponent :type "PrimitiveComponent Object Reference") (OtherActor :type "Actor Object Reference") (OtherComp :type "PrimitiveComponent Object Reference") (OtherBodyIndex :type Integer) (bFromSweep :type Boolean) (SweepResult :type "HitResult Structure (by ref)"))
  ; Stop direction
  (`self.StopMove` (3.0 0.0 0.0)))

(event `self.Box_stop_right.OnComponentBeginOverlap`
  (params (OverlappedComponent :type "PrimitiveComponent Object Reference") (OtherActor :type "Actor Object Reference") (OtherComp :type "PrimitiveComponent Object Reference") (OtherBodyIndex :type Integer) (bFromSweep :type Boolean) (SweepResult :type "HitResult Structure (by ref)"))
  ; Stop direction
  (`self.StopMove` (0.0 -3.0 0.0)))

(event `self.Box_stop_front.OnComponentBeginOverlap`
  (params (OverlappedComponent :type "PrimitiveComponent Object Reference") (OtherActor :type "Actor Object Reference") (OtherComp :type "PrimitiveComponent Object Reference") (OtherBodyIndex :type Integer) (bFromSweep :type Boolean) (SweepResult :type "HitResult Structure (by ref)"))
  ; Stop direction
  (`self.StopMove` (-3.0 0.0 0.0)))

(event `self.Box_stop_left.OnComponentBeginOverlap`
  (params (OverlappedComponent :type "PrimitiveComponent Object Reference") (OtherActor :type "Actor Object Reference") (OtherComp :type "PrimitiveComponent Object Reference") (OtherBodyIndex :type Integer) (bFromSweep :type Boolean) (SweepResult :type "HitResult Structure (by ref)"))
  ; Stop direction
  (`self.StopMove` (0.0 3.0 0.0)))

(fn `UserConstructionScript`)