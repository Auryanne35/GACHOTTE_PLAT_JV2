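; BP_fakePlatform is a fake platform that rotates its Arrow component when something begins overlapping its Box, then resets.
; A Rotation timeline lerps the Arrow's relative rotation from zero to Rotate, then reverses after a ten-second delay.
; The Good flag blocks retriggering until the reversal starts and stops the reverse pass's Finished event from looping.
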(event `self.Box.OnComponentBeginOverlap`
  (params (OverlappedComponent :type "PrimitiveComponent Object Reference") (OtherActor :type "Actor Object Reference") (OtherComp :type "PrimitiveComponent Object Reference") (OtherBodyIndex :type Integer) (bFromSweep :type Boolean) (SweepResult :type "HitResult Structure (by ref)"))
  (if (`self.good`)
    (set `self.good` false)
    (bind (_direction _newtrack_0) (`Timeline|Rotation` :!via `PlayFromStart` :!label _label)
      (:`Update`
        (`SceneComponent.K2_SetRelativeRotation` (`self.Arrow`) (`KismetMathLibrary.RLerp` (struct) (`self.rotate`) _newtrack_0) false false))
      (:`Finished`
        (if (not (`self.good`))
          (`KismetSystemLibrary.Delay` 10.0)
          (set `self.good` true)
          (goto _label :!via `ReverseFromEnd`))))))

(fn `UserConstructionScript`)